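; Player inventory component that handles item and money pickup, health values and their UI widgets.
; A per-tick forward sphere trace drives the interact prompt, and the interaction input adds the found item, destroys its actor and refreshes the inventory UI.
; Items live in fixed-size sword, shield and eatable arrays, stacking up to DataTable limits before taking empty slots.
; Capsule overlap collects money, and health functions update both health bars.
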(event EventBeginPlay
  (bind _allitems (Variables|Default|GetAllItems))
  (bind (_swords _shields _eatables) (Utilities|Struct|BreakS_AllItems _allitems))
  (Utilities|FlowControl|Sequence
    (:then_1
      (Input|AddMappingContext (PlayerController|LocalPlayerSubsystems|GetEnhancedInputLocalPlayerSubsystem (Game|GetPlayerController 0)) "/Game/inventory/InventoryFiles/inputs/inventoryInputs.inventoryInputs" 0 "(bIgnoreAllPressedKeysUntilRelease=True,bForceImmediately=False)")
      (bind _returnvalue (UserInterface|CreateWidget "/Game/inventory/InventoryFiles/UI/inventoryUI.inventoryUI_C"))
      (Variables|money|Setinventory%20widget _returnvalue)
      (bind _asbp_third_person_character (Utilities|Casting|CastToBP_ThirdPersonCharacter (Game|GetPlayerCharacter 0)))
      (bind _output_get (Variables|Default|Setplayer%20Character _asbp_third_person_character))
      (Collision|AssignOnComponentBeginOverlap (Variables|/Script/Engine.Character|GetCapsuleComponent _output_get) (EventDispatchers|CreateEvent :!event PickupMoney))
      (healthbar|HealthbarINT)
      (bind _returnvalue_2 (UserInterface|CreateWidget "/Game/inventory/InventoryFiles/UI/WBP_Interact.WBP_Interact_C"))
      (Variables|Default|SetinteractWidget _returnvalue_2)
      (Utilities|Array|Resize _swords 5)
      (Utilities|Array|Resize _shields 8)
      (Utilities|Array|Resize _eatables 7)
      (bind _asinventory_ui (Utilities|Casting|CastToinventoryUI (Variables|money|Getinventory%20widget)))
      (Default|UpdateItemsinInventoryUI _asinventory_ui (Variables|Default|GetAllItems)))))

(event EventTick
  (params (DeltaSeconds :type Float%20%28single-precision%29))
  (bind _interactwidget (Variables|Default|GetinteractWidget))
  (bind (_item _founditem) (CallFunction|TraceItemstoPickup))
  (Variables|/Game/inventory/InventoryFiles/UI/WBP_ItemInfo.WBP_ItemInfo_C|Setitem (Variables|/Game/inventory/InventoryFiles/UI/WBP_Interact.WBP_Interact_C|GetWBP_ItemInfo (Variables|Default|GetinteractWidget)) _item)
  (if _founditem
    (UserInterface|Viewport|AddtoViewport _interactwidget 0)
    (else
      (Widget|RemovefromParent _interactwidget))))

(event Input|EnhancedActionEvents|EnhancedInputActionIA_Inventory
  (params (ActionValue :type Boolean) (ElapsedSeconds :type Float%20%28double-precision%29) (TriggeredSeconds :type Float%20%28double-precision%29) (InputAction :type Input%20Action%20Object%20Reference :default "/Game/inventory/InventoryFiles/inputs/IA_Inventory.IA_Inventory"))
  (bind _returnvalue (Game|GetPlayerController 0))
  (:Triggered
    (UserInterface|Viewport|AddtoViewport (Variables|money|Getinventory%20widget) 0)
    (Variables|/Script/Engine.PlayerController|SetbShowMouseCursor _returnvalue true)
    (Input|SetInputModeUIOnly _returnvalue (Variables|money|Getinventory%20widget) "DoNotLock" false)))

(event Input|EnhancedActionEvents|EnhancedInputActionIA_Interaction
  (params (ActionValue :type Boolean) (ElapsedSeconds :type Float%20%28double-precision%29) (TriggeredSeconds :type Float%20%28double-precision%29) (InputAction :type Input%20Action%20Object%20Reference :default "/Game/inventory/InventoryFiles/inputs/IA_Interaction.IA_Interaction"))
  (:Triggered
    (bind (_item _founditem _actoritem) (CallFunction|TraceItemstoPickup))
    (if _founditem
      (bind _success (inventory|AddtoInventory _item))
      (if _success
        (Actor|DestroyActor _actoritem)
        (bind _asinventory_ui (Utilities|Casting|CastToinventoryUI (Variables|money|Getinventory%20widget)))
        (Default|UpdateItemsinInventoryUI _asinventory_ui (Variables|Default|GetAllItems))))))

(fn PickupMoney
  (params (OverlappedComponent :type Primitive%20Component%20Object%20Reference) (OtherActor :type Actor%20Object%20Reference) (OtherComp :type Primitive%20Component%20Object%20Reference) (OtherBodyIndex :type Integer) (bFromSweep :type Boolean) (SweepResult :type Hit%20Result%20Structure%20%28by%20ref%29))
  (bind _asbp_money_collect (Utilities|Casting|CastToBP_MoneyCollect OtherActor))
  (bind _returnvalue (Utilities|GetDataTableRow "/Game/inventory/InventoryFiles/structures/TD_Money.TD_Money" (.rowname (Variables|/Game/inventory/InventoryFiles/BluePrints/BP_MoneyCollect.BP_MoneyCollect_C|GetMoney _asbp_money_collect)))
    (:then
      (Variables|moneyAmount|Setmoney%20AmountComponent (+ (.amount _returnvalue) (Variables|moneyAmount|Getmoney%20AmountComponent)))
      (Variables|/Game/inventory/InventoryFiles/UI/inventoryUI.inventoryUI_C|SetmoneyAmountWidget (Variables|money|Getinventory%20widget) (Variables|moneyAmount|Getmoney%20AmountComponent))
      (Actor|DestroyActor _asbp_money_collect)
      (return))))

(fn IncreaseHealth
  (params (health%20to%20increase :type Float%20%28double-precision%29))
  (Variables|healthbar|Sethealth (+ health%20to%20increase (Variables|healthbar|Gethealth)))
  (Default|UpdateHealthBar (Variables|Default|Gethealthbar%20widget))
  (Default|UpdateHealthBar (Variables|/Game/inventory/InventoryFiles/UI/inventoryUI.inventoryUI_C|GetWBP_HealthBar (Variables|money|Getinventory%20widget))))

(fn DecreseHealth
  (params (health%20to%20decrease :type Float%20%28double-precision%29))
  (Variables|healthbar|Sethealth (- health%20to%20decrease (Variables|healthbar|Gethealth)))
  (Default|UpdateHealthBar (Variables|Default|Gethealthbar%20widget))
  (Default|UpdateHealthBar (Variables|/Game/inventory/InventoryFiles/UI/inventoryUI.inventoryUI_C|GetWBP_HealthBar (Variables|money|Getinventory%20widget))))

(fn HealthbarINT
  (bind _returnvalue (UserInterface|CreateWidget "/Game/inventory/InventoryFiles/UI/WBP_HealthBar.WBP_HealthBar_C"))
  (bind _output_get (Variables|Default|Sethealthbar%20widget _returnvalue))
  (Class|UserWidget|SetPositioninViewport _output_get "(X=5.000000,Y=5.000000)" true)
  (UserInterface|Viewport|AddtoViewport _output_get 0))

(fn TraceItemstoPickup
  (bind _returnvalue (Game|GetPlayerCharacter 0))
  (bind _returnvalue_2 (Transformation|GetActorLocation _returnvalue))
  (bind _returnvalue_3 (- _returnvalue_2 "0.000000,0.000000,60.000000"))
  (bind _outhit (Collision|SphereTraceByChannel _returnvalue_3 (+ (* (Transformation|GetActorForwardVector _returnvalue) 1.2e+02) _returnvalue_3) 3e+01 "TraceTypeQuery1" false 0 "ForOneFrame"))
  (bind _asbp_item (Utilities|Casting|CastToBP_item (.hitactor _outhit))
    (:then
      (return (Variables|/Game/inventory/InventoryFiles/BluePrints/BP_item.BP_item_C|Getitems _asbp_item) true (.hitactor _outhit)))
    (:CastFailed
      (return "" false 0))))

(fn AddtoInventory
  (params (item :type S%20Slot%20Structure))
  (bind (_itemid _itemtype) (Utilities|Struct|BreakS_Slot item))
  (bind (_itemid_2 _itemtype_2 _quantity) (Utilities|Struct|BreakS_Slot item))
  (bind (_itemid_3 _itemtype_3) (Utilities|Struct|BreakS_Slot item))
  (bind (_itemid_4 _itemtype_4 _quantity_2) (Utilities|Struct|BreakS_Slot item))
  (bind (_itemid_5 _itemtype_5) (Utilities|Struct|BreakS_Slot item))
  (bind (_itemid_6 _itemtype_6 _quantity_3) (Utilities|Struct|BreakS_Slot item))
  (switch Utilities|FlowControl|Switch|SwitchonE_itemTypes (.itemtype (Utilities|Struct|BreakS_Slot item))
    (:NewEnumerator0
      (for (_array_element _array_index) (.swords (Utilities|Struct|BreakS_AllItems (Variables|Default|GetAllItems)))
        (if (== (.RowName (Utilities|Struct|BreakDataTableRowHandle (.itemID (Utilities|Struct|BreakS_Slot _array_element)))) (.RowName (Utilities|Struct|BreakDataTableRowHandle (.itemID (Utilities|Struct|BreakS_Slot item)))))
          (bind _returnvalue (Utilities|GetDataTableRow "/Game/inventory/InventoryFiles/structures/DT_Items.DT_Items" (.RowName (Utilities|Struct|BreakDataTableRowHandle _itemid_6)))
            (:then
              (if (>= (.stacksize (Utilities|Struct|BreakS_items _returnvalue)) (+ _quantity_3 (.quantity (Utilities|Struct|BreakS_Slot _array_element))))
                (Utilities|Array|SetArrayElem (.swords (Utilities|Struct|BreakS_AllItems (Variables|Default|GetAllItems))) _array_index (Utilities|Struct|MakeS_Slot _itemid _itemtype (+ _quantity_3 (.quantity (Utilities|Struct|BreakS_Slot _array_element)))))
                (return true))))))
      (for (_array_element_2 _array_index_2) (.swords (Utilities|Struct|BreakS_AllItems (Variables|Default|GetAllItems)))
        (if (== (.quantity (Utilities|Struct|BreakS_Slot _array_element_2)) 0)
          (Utilities|Array|SetArrayElem (.swords (Utilities|Struct|BreakS_AllItems (Variables|Default|GetAllItems))) _array_index_2 item)
          (return true)))
      (return false))
    (:NewEnumerator1
      (for (_array_element_3 _array_index_3) (.shields (Utilities|Struct|BreakS_AllItems (Variables|Default|GetAllItems)))
        (if (== (.RowName (Utilities|Struct|BreakDataTableRowHandle (.itemID (Utilities|Struct|BreakS_Slot _array_element_3)))) (.RowName (Utilities|Struct|BreakDataTableRowHandle (.itemID (Utilities|Struct|BreakS_Slot item)))))
          (bind _returnvalue_2 (Utilities|GetDataTableRow "/Game/inventory/InventoryFiles/structures/DT_Items.DT_Items" (.RowName (Utilities|Struct|BreakDataTableRowHandle _itemid_4)))
            (:then
              (if (>= (.stacksize (Utilities|Struct|BreakS_items _returnvalue_2)) (+ _quantity_2 (.quantity (Utilities|Struct|BreakS_Slot _array_element_3))))
                (Utilities|Array|SetArrayElem (.shields (Utilities|Struct|BreakS_AllItems (Variables|Default|GetAllItems))) _array_index_3 (Utilities|Struct|MakeS_Slot _itemid_5 _itemtype_5 (+ _quantity_2 (.quantity (Utilities|Struct|BreakS_Slot _array_element_3)))))
                (return true))))))
      (for (_array_element_4 _array_index_4) (.shields (Utilities|Struct|BreakS_AllItems (Variables|Default|GetAllItems)))
        (if (== (.quantity (Utilities|Struct|BreakS_Slot _array_element_4)) 0)
          (Utilities|Array|SetArrayElem (.shields (Utilities|Struct|BreakS_AllItems (Variables|Default|GetAllItems))) _array_index_4 item)
          (return true)))
      (return false))
    (:NewEnumerator2
      (for (_array_element_5 _array_index_5) (.eatables (Utilities|Struct|BreakS_AllItems (Variables|Default|GetAllItems)))
        (if (== (.RowName (Utilities|Struct|BreakDataTableRowHandle (.itemID (Utilities|Struct|BreakS_Slot _array_element_5)))) (.RowName (Utilities|Struct|BreakDataTableRowHandle (.itemID (Utilities|Struct|BreakS_Slot item)))))
          (bind _returnvalue_3 (Utilities|GetDataTableRow "/Game/inventory/InventoryFiles/structures/DT_Items.DT_Items" (.RowName (Utilities|Struct|BreakDataTableRowHandle _itemid_2)))
            (:then
              (if (>= (.stacksize (Utilities|Struct|BreakS_items _returnvalue_3)) (+ _quantity (.quantity (Utilities|Struct|BreakS_Slot _array_element_5))))
                (Utilities|Array|SetArrayElem (.eatables (Utilities|Struct|BreakS_AllItems (Variables|Default|GetAllItems))) _array_index_5 (Utilities|Struct|MakeS_Slot _itemid_3 _itemtype_3 (+ _quantity (.quantity (Utilities|Struct|BreakS_Slot _array_element_5)))))
                (return true))))))
      (for (_array_element_6 _array_index_6) (.eatables (Utilities|Struct|BreakS_AllItems (Variables|Default|GetAllItems)))
        (if (== (.quantity (Utilities|Struct|BreakS_Slot _array_element_6)) 0)
          (Utilities|Array|SetArrayElem (.eatables (Utilities|Struct|BreakS_AllItems (Variables|Default|GetAllItems))) _array_index_6 item)
          (return true)))
      (return false))))