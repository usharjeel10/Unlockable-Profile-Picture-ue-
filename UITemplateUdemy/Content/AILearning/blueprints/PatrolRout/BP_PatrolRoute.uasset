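; BP_PatrolRoute is a patrol route actor that supplies waypoints from the points of its spline.
; IncrementPatrolPath steps the patrol index by the current direction, flipping direction at the first and last points for a back-and-forth loop.
; GetCurrentSplineWorlLocation returns the world-space location of the spline point at the current index.
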(event Custom|IncrementPatrolPath
  (bind _output_get (Variables|Default|SetpatrolIndex (+ (Variables|Default|GetpatrolIndex) (Variables|Default|Getdirection))))
  (if (== _output_get (- (Spline|GetNumberOfSplinePoints (Variables|Default|GetSpline)) 1))
    (Variables|Default|Setdirection -1)
    (elif (== (Variables|Default|GetpatrolIndex) 0)
      (Variables|Default|Setdirection 1))))

(fn ConstructionScript)

(fn GetCurrentSplineWorlLocation
  (return (Spline|GetLocationatSplinePoint (Variables|Default|GetSpline) (Variables|Default|GetpatrolIndex) "World")))