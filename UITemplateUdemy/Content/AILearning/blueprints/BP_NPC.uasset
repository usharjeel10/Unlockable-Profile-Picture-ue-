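; BP_NPC is an AI character that can carry a patrol route, equip a sword and perform a melee attack.
; Attack plays a mutant swipe montage and fires OnAttackEnd whether it completes or is interrupted.
; WeiredSword spawns a BP_Sword on the left-hand socket and flags the weapon as attached.
; GetPatrolRoute exposes the route reference, while SetMovementSpeed is a stub that ignores its input and returns zero.
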(event Custom|Attack
  (Animation|Montage|PlayMontage (Variables|Character|GetMesh) "/Game/Characters/Mannequins/Animations/Mixamo/Attack/MutantSwiping_UE_Montage.MutantSwiping_UE_Montage"
    (:OnCompleted
      _)
    (:OnInterrupted
      _))
  (Default|CallOnAttackEnd))

(event Custom|WeiredSword
  (bind _returnvalue (Game|SpawnActorfromClass "/Game/AILearning/blueprints/weapons/BP_Sword.BP_Sword_C" (Transformation|GetActorTransform) "AlwaysSpawn" "MultiplyWithRoot" 0 0))
  (Transformation|AttachComponentToComponent _returnvalue (Variables|Character|GetMesh) "hand_lSocket" "SnapToTarget" "SnapToTarget" "SnapToTarget" true)
  (Variables|Default|SetIsWeaponAttached true))

(event EventBeginPlay)

(fn ConstructionScript)

(fn GetPatrolRoute
  (return (Variables|Default|GetpatrolRouteRef)))

(fn SetMovementSpeed
  (params (Speed :type NPC_SpeedEnum%20Enum :default "NewEnumerator0"))
  (return 0.0))